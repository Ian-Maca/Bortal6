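; BP_ItemPickup is a spinning laser ammo pickup for the first-person character.
; BeginPlay colors the mesh's spokes material by ammo type (Pop, Push, Gravity or Pull) and starts the Rocking timeline.
; Tick spins the mesh in world and local yaw, with the timeline's Roll value driving a pitch rocking motion.
; Capsule overlap passes ammo type and amount to the character and destroys the pickup, only while the game mode reports a held laser.
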(event `self.ReceiveBeginPlay`
  (bind _asbortal_game_mode (cast `BortalGameMode` (`GameplayStatics.GetGameMode`)))
  (set `self.As Bortal Game Mode` _asbortal_game_mode)
  (`self.Set Color`)
  (bind (_direction _roll) (`Timeline|Rocking`)))

(event `self.ReceiveTick`
  (params (DeltaSeconds :type "Float (single-precision)"))
  (bind _mesh (`self.mesh`))
  (`SceneComponent.K2_AddWorldRotation` _mesh (`KismetMathLibrary.MakeRotator` 0.0 (* DeltaSeconds (stale `self.ReceiveBeginPlay` _roll)) (* DeltaSeconds 80.0)) false false)
  (`SceneComponent.K2_AddLocalRotation` _mesh (`KismetMathLibrary.MakeRotator` 0.0 0.0 (* DeltaSeconds 10.0)) false false))

(event `self.Capsule.OnComponentBeginOverlap`
  (params (OverlappedComponent :type "PrimitiveComponent Object Reference") (OtherActor :type "Actor Object Reference") (OtherComp :type "PrimitiveComponent Object Reference") (OtherBodyIndex :type Integer) (bFromSweep :type Boolean) (SweepResult :type "HitResult Structure (by ref)"))
  (if (`BortalGameMode.bIsHoldingLaser` (`self.As Bortal Game Mode`))
    (bind _asbp_first_person_character (cast `/Game/FirstPerson/Blueprints/BP_FirstPersonCharacter` OtherActor))
    (`/Game/FirstPerson/Blueprints/BP_FirstPersonCharacter.Item Pickup` _asbp_first_person_character (`self.AmmoType`) (`self.AmmoAmount`))
    (`self.K2_DestroyActor`)))

(fn `Set Color`
  (bind _mesh (`self.mesh`))
  (switch `string` (`self.AmmoType`)
    (:`Pop`
      (`PrimitiveComponent.SetMaterialByName` _mesh "spokes" "/Game/Mine/Materials/M_PopLaser.M_PopLaser"))
    (:`Push`
      (`PrimitiveComponent.SetMaterialByName` _mesh "spokes" "/Game/Mine/Materials/M_PushLaser.M_PushLaser"))
    (:`Gravity`
      (`PrimitiveComponent.SetMaterialByName` _mesh "spokes" "/Game/Mine/Materials/M_GravLaser.M_GravLaser"))
    (:`Pull`
      (`PrimitiveComponent.SetMaterialByName` _mesh "spokes" "/Game/Mine/Materials/M_PullLaser.M_PullLaser"))))

(fn `UserConstructionScript`)