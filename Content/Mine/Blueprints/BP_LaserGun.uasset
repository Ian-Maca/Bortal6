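; Laser gun with four switchable modes (Push, Gravity/Slow, Pop, Pull) that act on BP_ItemTemplate actors.
; Number keys switch modes that have ammo, swapping the gun material, while the laser is held.
; Releasing shoot spends ammo, briefly shows the beam and line-traces from the muzzle, passing mode and direction to the hit item's BeenShot.
; BortalGameMode handles ammo use and per-mode material lerp, which the gun caches and applies as scalar parameters.
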(event `EnhancedInput|/Game/FirstPerson/Input/Actions/IA_KeyOne`
  (params (ActionValue :type Boolean) (ElapsedSeconds :type "Float (double-precision)") (TriggeredSeconds :type "Float (double-precision)") (InputAction :type "InputAction Object Reference" :default "/Game/FirstPerson/Input/Actions/IA_KeyOne.IA_KeyOne"))
  (:`Triggered`
    (if (> (`self.pushAmmo`) 0)
      (`self.Update Laser Type` 0))))

(event `EnhancedInput|/Game/FirstPerson/Input/Actions/IA_KeyTwo`
  (params (ActionValue :type Boolean) (ElapsedSeconds :type "Float (double-precision)") (TriggeredSeconds :type "Float (double-precision)") (InputAction :type "InputAction Object Reference" :default "/Game/FirstPerson/Input/Actions/IA_KeyTwo.IA_KeyTwo"))
  (:`Triggered`
    (if (> (`self.gravAmmo`) 0)
      (`self.Update Laser Type` 1))))

(event `EnhancedInput|/Game/FirstPerson/Input/Actions/IA_KeyThree`
  (params (ActionValue :type Boolean) (ElapsedSeconds :type "Float (double-precision)") (TriggeredSeconds :type "Float (double-precision)") (InputAction :type "InputAction Object Reference" :default "/Game/FirstPerson/Input/Actions/IA_KeyThree.IA_KeyThree"))
  (:`Triggered`
    (if (> (`self.popAmmo`) 0)
      (`self.Update Laser Type` 2))))

(event `EnhancedInput|/Game/IA_KeyFour`
  (params (ActionValue :type Boolean) (ElapsedSeconds :type "Float (double-precision)") (TriggeredSeconds :type "Float (double-precision)") (InputAction :type "InputAction Object Reference" :default "/Game/IA_KeyFour.IA_KeyFour"))
  (:`Triggered`
    (if (> (`self.pullAmmo`) 0)
      (`self.Update Laser Type` 3))))

(event `self.ReceiveBeginPlay`
  (bind _asbortal_game_mode (cast `BortalGameMode` (`GameplayStatics.GetGameMode`)))
  (bind _output_get (set `self.GameModeRef` _asbortal_game_mode))
  (set `self.pushAmmo` (`BortalGameMode.PushLaserEnergy` _output_get))
  (set `self.popAmmo` (`BortalGameMode.PopLaserEnergy` _output_get))
  (set `self.gravAmmo` (`BortalGameMode.GravLaserEnergy` _output_get)))

(event `EnhancedInput|/Game/FirstPerson/Input/Actions/IA_Shoot`
  (params (ActionValue :type Boolean) (ElapsedSeconds :type "Float (double-precision)") (TriggeredSeconds :type "Float (double-precision)") (InputAction :type "InputAction Object Reference" :default "/Game/FirstPerson/Input/Actions/IA_Shoot.IA_Shoot"))
  (bind _nuzzlemarker (`self.nuzzleMarker`))
  (bind _lasertye (`self.LaserTye`))
  (bind _returnvalue (`SceneComponent.K2_GetComponentLocation` _nuzzlemarker))
  (:`Completed`
    (if (`BortalGameMode.bIsHoldingLaser` (`self.GameModeRef`))
      (bind _curlaserempty (`self.NoAmmo`))
      (if (not _curlaserempty)
        (`self.DecrementLaserFuel`)
        (bind (_outhit _returnvalue_2) (`KismetSystemLibrary.LineTraceSingle` :`Start` _returnvalue :`End` (+ _returnvalue (* (`SceneComponent.GetForwardVector` _nuzzlemarker) (`self.traceDistance`))) :`TraceChannel` "TraceTypeQuery1" :`DrawTime` 0.0))
        (`self.QuickLaser`)
        (if _returnvalue_2
          (bind _asbp_item_template (cast `/Game/Mine/Blueprints/BP_ItemTemplate` (`.HitActor` (`GameplayStatics.BreakHitResult` _outhit))))
          (`/Engine/EditorBlueprintResources/StandardMacros.IsValid` _asbp_item_template
            (:`Is Valid`
              (`/Game/Mine/Blueprints/BP_ItemTemplate.BeenShot` _asbp_item_template _lasertye (`self.GetActorForwardVector` self))
              (`KismetSystemLibrary.PrintString` (`|GetEnumeratorNameAsString` _lasertye)))))))))

(fn `DecrementLaserFuel`
  (bind _gamemoderef (`self.GameModeRef`))
  (bind _returnvalue (`KismetMathLibrary.Conv_IntToByte` 5))
  (switch `ELaserType` (`self.LaserTye`)
    (:`Push`
      (bind _returnvalue_2 (`BortalGameMode.PushUseAmmo` _gamemoderef _returnvalue))
      (set `self.pushAmmo` _returnvalue_2))
    (:`Slow`
      (bind _returnvalue_3 (`BortalGameMode.GravUseAmmo` _gamemoderef _returnvalue))
      (set `self.gravAmmo` _returnvalue_3))
    (:`Pop`
      (bind _returnvalue_4 (`BortalGameMode.PopUseAmmo` _gamemoderef _returnvalue))
      (set `self.popAmmo` _returnvalue_4))
    (:`Pull`
      (bind _returnvalue_5 (`BortalGameMode.PullUseAmmo` _gamemoderef _returnvalue))
      (set `self.pullAmmo` _returnvalue_5))))

(fn `LaserOff`
  (`SceneComponent.SetVisibility` (`self.NS_Beam`) false false))

(fn `NoAmmo`
  (returns (CurLaserEmpty :type Boolean))
  (locals (return :type Boolean :default false))
  (switch `ELaserType` (`self.LaserTye`)
    (:`Push`
      (if (== (`self.pushAmmo`) 0)
        (set `local.return` true)
        (else
          (set `local.return` false))))
    (:`Slow`
      (if (== 0 (`self.gravAmmo`))
        (set `local.return` true)
        (else
          (set `local.return` false))))
    (:`Pop`
      (if (== 0 (`self.popAmmo`))
        (set `local.return` true)
        (else
          (set `local.return` false))))
    (:`Pull`
      (if (== (`self.pullAmmo`) 0)
        (set `local.return` true)
        (else
          (set `local.return` false)))))
  (return (`local.return`)))

(fn `QuickLaser`
  (bind _gunmesh (`self.GunMesh`))
  (bind _gamemoderef (`self.GameModeRef`))
  (`SceneComponent.SetVisibility` (`self.NS_Beam`) true false)
  (`KismetSystemLibrary.K2_SetTimer` null "LaserOff" 0.1)
  (switch `ELaserType` (`self.LaserTye`)
    (:`Push`
      (bind _returnvalue (`BortalGameMode.MatLerpIncrement` _gamemoderef 0.05))
      (bind _output_get (set `self.PushMatLerp` _returnvalue))
      (`MeshComponent.SetScalarParameterValueOnMaterials` _gunmesh "Cum" _output_get)
      (`KismetSystemLibrary.PrintString` (`KismetStringLibrary.Conv_DoubleToString` _output_get)))
    (:`Slow`
      (bind _returnvalue_2 (`BortalGameMode.GravityMatLerpIncrement` _gamemoderef 0.05))
      (bind _output_get_2 (set `self.GravMatLerp` _returnvalue_2))
      (`MeshComponent.SetScalarParameterValueOnMaterials` _gunmesh "Jizz" _output_get_2)
      (`KismetSystemLibrary.PrintString` (`KismetStringLibrary.Conv_DoubleToString` _output_get_2)))
    (:`Pop`
      (bind _returnvalue_3 (`BortalGameMode.PopMatLerpIncrement` _gamemoderef 0.05))
      (bind _output_get_3 (set `self.PopMatLerp` _returnvalue_3))
      (`MeshComponent.SetScalarParameterValueOnMaterials` _gunmesh "Piss" _output_get_3)
      (`KismetSystemLibrary.PrintString` (`KismetStringLibrary.Conv_DoubleToString` _output_get_3)))
    (:`Pull`
      (bind _returnvalue_4 (`BortalGameMode.PullMatLerpIncrement` _gamemoderef 0.05))
      (bind _output_get_4 (set `self.PullMatLerp` _returnvalue_4))
      (`MeshComponent.SetScalarParameterValueOnMaterials` _gunmesh "Ejac" _output_get_4)
      (`KismetSystemLibrary.PrintString` (`KismetStringLibrary.Conv_DoubleToString` _output_get_4)))))

(fn `Update Laser Type`
  (params (Index :type Integer))
  (locals (PushMode :type Byte) (SlowMode :type Byte :default 1) (PopMode :type Byte :default 2) (PullMode :type Byte :default 3))
  (bind _gunmesh (`self.GunMesh`))
  ;[1 1 1] Switch Laser Types
  (switch `int` Index
    (:`0`
      (if (and (!= (`self.LaserTye`) (`local.PushMode`)) (`BortalGameMode.bIsHoldingLaser` (`self.GameModeRef`)))
        (set `self.LaserTye` "Push")
        (`PrimitiveComponent.SetMaterial` _gunmesh 0 "/Game/Mine/Materials/M_PushLaser.M_PushLaser")
        (`MeshComponent.SetScalarParameterValueOnMaterials` _gunmesh "Cum" (`self.PushMatLerp`))
        (`KismetSystemLibrary.PrintString` "Set Laser to: \"Push\"")))
    (:`1`
      (if (and (`BortalGameMode.bIsHoldingLaser` (`self.GameModeRef`)) (!= (`self.LaserTye`) (`local.SlowMode`)))
        (set `self.LaserTye` "Slow")
        (`PrimitiveComponent.SetMaterial` (`self.GunMesh`) 0 "/Game/Mine/Materials/M_GravLaser.M_GravLaser")
        (`MeshComponent.SetScalarParameterValueOnMaterials` _gunmesh "Jizz" (`self.GravMatLerp`))
        (`KismetSystemLibrary.PrintString` "Set Laser to: \"Gravity\"")))
    (:`2`
      (if (and (`BortalGameMode.bIsHoldingLaser` (`self.GameModeRef`)) (!= (`self.LaserTye`) (`local.PopMode`)))
        (set `self.LaserTye` "Pop")
        (`PrimitiveComponent.SetMaterial` (`self.GunMesh`) 0 "/Game/Mine/Materials/M_PopLaser.M_PopLaser")
        (`MeshComponent.SetScalarParameterValueOnMaterials` _gunmesh "Piss" (`self.PopMatLerp`))
        (`KismetSystemLibrary.PrintString` "Set Laser to: \"Pop\"")))
    (:`3`
      (if (and (`BortalGameMode.bIsHoldingLaser` (`self.GameModeRef`)) (!= (`self.LaserTye`) (`local.PullMode`)))
        (set `self.LaserTye` "Pull")
        (`PrimitiveComponent.SetMaterial` (`self.GunMesh`) 0 "/Game/Mine/Materials/M_PullLaser.M_PullLaser")
        (`MeshComponent.SetScalarParameterValueOnMaterials` _gunmesh "Ejac" (`self.PullMatLerp`))
        (`KismetSystemLibrary.PrintString` "Set Laser to: \"Pul\"")))))

(fn `UserConstructionScript`)